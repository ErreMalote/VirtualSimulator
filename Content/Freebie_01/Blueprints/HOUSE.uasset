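; HOUSE is a configurable modular building Blueprint whose construction script varies its look and height, with no active event logic.
; It tints the windows through a dynamic material instance and picks a plaster or awning material for the main mesh.
; Toggles remove the Box component and swing shutters open at random angles.
; Storeys raises the roof and destroys unused mid-storey components.
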(event `self.ReceiveBeginPlay`)

(event `self.ReceiveActorBeginOverlap`
  (params (OtherActor :type "Actor Object Reference")))

(event `self.ReceiveTick`
  (params (DeltaSeconds :type "Float (single-precision)")))

(fn `UserConstructionScript`
  (bind _main_6x6_mdl (`self.Main_6x6_mdl`))
  (bind _storeys (`self.Storeys`))
  (bind _mid_storey_4 (`self.Mid_Storey_4`))
  (bind _returnvalue (`PrimitiveComponent.CreateDynamicMaterialInstance` _main_6x6_mdl 2 "/Game/MedievalVillage/Materials/Window_Inst.Window_Inst"))
  (`MaterialInstanceDynamic.SetVectorParameterValue` _returnvalue "Tint" (`KismetMathLibrary.Conv_VectorToLinearColor` (`self.Tint`)))
  (`PrimitiveComponent.SetMaterial` _main_6x6_mdl 0 (`KismetArrayLibrary.Array_Get` (`|MakeArray` "/Game/MedievalVillage/Materials/Plaster_B_Inst.Plaster_B_Inst" "/Game/MedievalVillage/Materials/Plaster_C_Inst.Plaster_C_Inst" "/Game/MedievalVillage/Materials/Plaster_Inst.Plaster_Inst" "/Game/MedievalVillage/Materials/Awning_VarB_Inst.Awning_VarB_Inst" :!type "MaterialInterface Object Reference") (`self.Plaster`)))
  (if (`self.Door Toggle`)
    (`ActorComponent.K2_DestroyComponent` (`self.Box`)))
  (if (`self.ShuttersOpen`)
    (`SceneComponent.K2_AddLocalRotation` (`|MakeArray` (`self.Shutter_Left_1`) (`self.Shutter_Left_2`) :!type "SceneComponent Object Reference") (`KismetMathLibrary.MakeRotator` 0.0 0.0 (`KismetMathLibrary.RandomFloatInRange` 150.0 180.0)) false false)
    (`SceneComponent.K2_AddLocalRotation` (`|MakeArray` (`self.Shutter_Right_1`) (`self.Shutter_Right_2`) :!type "SceneComponent Object Reference") (`KismetMathLibrary.MakeRotator` 0.0 0.0 (`KismetMathLibrary.RandomFloatInRange` -150.0 -180.0)) false false))
  (`SceneComponent.K2_AddWorldTransform` (`self.Roof_6x6`) (`KismetMathLibrary.Conv_VectorToTransform` (`KismetMathLibrary.MakeVector` 0.0 0.0 (* _storeys 300.0))) false false)
  (if (< _storeys 4)
    (`ActorComponent.K2_DestroyComponent` _mid_storey_4)
    (`ActorComponent.K2_DestroyComponent` (`self.Mid_Storey_4`))
    (`ActorComponent.K2_DestroyComponent` (`SceneComponent.GetChildrenComponents` _mid_storey_4 false)))
  (if (< _storeys 3)
    (`ActorComponent.K2_DestroyComponent` (`self.Mid_Storey_3`)))
  (if (< _storeys 2)
    (`ActorComponent.K2_DestroyComponent` (`self.Mid_Storey_2`))))