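; Modular straight top-floor building piece that varies its left and right windows and blinds at construction time.
; The Construction Script, when RandomBlinds is set, gives each blind a random vertical scale.
; When OpenWindows is set, it raises each window by a random world-space Z offset.
; Randomness is unseeded and re-rolls whenever construction reruns; the event graph holds only disabled stubs.
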(event `self.ReceiveBeginPlay`)

(event `self.ReceiveActorBeginOverlap`
  (params (OtherActor :type "Actor Object Reference")))

(event `self.ReceiveTick`
  (params (DeltaSeconds :type "Float (single-precision)")))

(fn `UserConstructionScript`
  (if (`self.Random Blinds `)
    (`SceneComponent.SetWorldScale3D` (`self.Blinds_L`) (`KismetMathLibrary.MakeVector` 0.94 1.0 (`KismetMathLibrary.RandomFloatInRange` 0.2 1.0)))
    (`SceneComponent.SetWorldScale3D` (`self.Blinds_R`) (`KismetMathLibrary.MakeVector` 0.94 1.0 (`KismetMathLibrary.RandomFloatInRange` 0.2 1.0))))
  (if (`self.Open Windows`)
    (`SceneComponent.K2_AddWorldOffset` (`self.Window_L`) (`KismetMathLibrary.MakeVector` 0.0 0.0 (`KismetMathLibrary.RandomFloatInRange` 50.0 70.0)) false false)
    (`SceneComponent.K2_AddWorldOffset` (`self.Window_R`) (`KismetMathLibrary.MakeVector` 0.0 0.0 (`KismetMathLibrary.RandomFloatInRange` 50.0 70.0)) false false)))